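; Base enemy Blueprint that wires up and toggles a floating health bar widget above the enemy.
; On BeginPlay it casts the HealthBar component's widget to EnemyHealthBarBP, passes itself as the owning Enemy, and hides it.
; ShowHealthBar makes the widget visible and then calls the parent implementation, while HideHealthBar only hides it again.
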(event `self.ReceiveBeginPlay`
  (bind _asenemy_health_bar_bp (cast `/Game/_Game_/HUD/EnemyHealthBarBP` (`WidgetComponent.GetUserWidgetObject` (`self.HealthBar`))))
  (set `/Game/_Game_/HUD/EnemyHealthBarBP.Enemy` self _asenemy_health_bar_bp)
  (`Widget.SetVisibility` (`WidgetComponent.GetUserWidgetObject` (`self.HealthBar`)) "Hidden"))

(event `self.ShowHealthBar`
  (`Widget.SetVisibility` (`WidgetComponent.GetUserWidgetObject` (`self.HealthBar`)) "Visible")
  (`parent.ShowHealthBar`))

(event `self.HideHealthBar`
  (`Widget.SetVisibility` (`WidgetComponent.GetUserWidgetObject` (`self.HealthBar`)) "Hidden"))

(fn `UserConstructionScript`)